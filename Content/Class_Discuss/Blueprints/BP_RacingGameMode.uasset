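; Game mode for a lap-based race, running the countdown, lap counting, race completion and UI.
; On BeginPlay it binds to the level's single expected starting line and its own race event dispatchers, then starts a looping countdown timer that fires race start.
; Starting line passes drive lap and race completion events.
; Helper functions record lap times through a timer component, print lap and total times, and manage the HUD and completion menu.
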(event `self.ReceiveBeginPlay`
  (`|ExecutionSequence`
    (:`then_0`
      ; Bind to Starting Line
      (bind (_startingline _bsuccess) (`self.GetStartingLine`))
      (if _bsuccess
        (add `/Game/Class_Discuss/Blueprints/BP_Startingline.OnStartingLinePassed` _startingline (`|CreateDelegate` :!event `OnStartingLinePassed`))
        (add `self.OnLapCompleted` (`|CreateDelegate` :!event `RecordLapTime`))))
    (:`then_1`
      ; Bind to Race Completed
      (add `self.OnRaceCompleted` (`|CreateDelegate` :!event `DisplayTimes`))
      (add `self.OnRaceCompleted` (`|CreateDelegate` :!event `DrawRaceCompleteMenu`))
      (add `self.OnRaceCompleted` (`|CreateDelegate` :!event `RemoveHUD`))
      (add `self.OnRaceCompleted` (`|CreateDelegate` :!event `Stop Timer`)))
    (:`then_2`
      ; HUD and Timer
      (add `self.OnRaceStarted` (`|CreateDelegate` :!event `DrawHUD`))
      (add `self.OnRaceStarted` (`|CreateDelegate` :!event `StartTimer`)))
    (:`then_3`
      ; Start Countdown
      (bind _returnvalue (`KismetSystemLibrary.K2_SetTimerDelegate` (`|CreateDelegate` :!event `Count Down`) 1.0 true))
      (set `self.CountdownTimerHandle` _returnvalue)
      (bind _returnvalue_2 (`|CreateWidget` "/Game/Class_Discuss/Blueprints/UI/WBP_Countdown.WBP_Countdown_C"))
      (`UserWidget.AddToViewport` _returnvalue_2 0))))

(event `OnStartingLinePassed`
  (params (LapCompleted :type Boolean))
  ; Starting Line Passed
  (if LapCompleted
    (bind _result (`/Engine/EditorBlueprintResources/StandardMacros.IncrementInt` (`self.LapsCompleted`))
      (:`  `
        (if (>= _result (`self.LapstoCompleteRace`))
          (`self.OnLapCompleted`)
          (`self.OnRaceCompleted`)
          (`KismetSystemLibrary.PrintString` "Race Completed!")
          (else
            (`self.OnLapCompleted`)
            (`KismetSystemLibrary.PrintString` "Lap Completed!")))))))

(event `Stop Timer`
  ; Stop Timer
  (`/Game/Class_Discuss/Blueprints/BP_Timer.StopTimer` (`self.BP_Timer`) false))

(event `StartTimer`
  ; Stop Timer
  (`/Game/Class_Discuss/Blueprints/BP_Timer.StartTimer` (`self.BP_Timer`) true))

(event `Count Down`
  ; Countdown
  (bind _result (`/Engine/EditorBlueprintResources/StandardMacros.DecrementInt` (`self.CountdownLength`))
    (:`  `
      (if (<= _result 0)
        (`self.OnRaceStarted`)
        (`KismetSystemLibrary.K2_ClearAndInvalidateTimerHandle` (`self.CountdownTimerHandle`))))))

(fn `DisplayTimes`
  (locals (TotalRaceTime :type "Float (double-precision)") (LapTime :type "Float (double-precision)"))
  (set `local.TotalRaceTime` 0.0)
  (for (_array_element _array_index) (`self.LapTimes`)
    (set `local.LapTime` _array_element)
    (`|ExecutionSequence`
      (:`then_0`
        ; Increment Time
        (set `local.TotalRaceTime` (+ (`local.TotalRaceTime`) (`local.LapTime`))))
      (:`then_1`
        ; Display Time
        (`KismetSystemLibrary.PrintString` (`KismetStringLibrary.Concat_StrStr` "Lap " (`KismetStringLibrary.Conv_IntToString` (+ _array_index 1)) ": " (`.AsString` (`/Game/Class_Discuss/Blueprints/BP_Timer.SecondsToTimeCode` (`self.BP_Timer`) (`local.LapTime`))))))))
  ; Dispay Total Race Time
  (`KismetSystemLibrary.PrintString` (`KismetStringLibrary.Concat_StrStr` "Total Time " (`.AsString` (`/Game/Class_Discuss/Blueprints/BP_Timer.SecondsToTimeCode` (`self.BP_Timer`) (`local.TotalRaceTime`)))) true true (struct :`G` 0.66 :`B` 1.0 :`A` 1.0) 10.0))

(fn `DrawHUD`
  (`/Engine/EditorBlueprintResources/StandardMacros.IsValid` (`self.RacingHUD`)
    (:`Is Valid`
      _)
    (:`Is Not Valid`
      (bind _returnvalue (`|CreateWidget` "/Game/Class_Discuss/Blueprints/UI/WBP_RacingHUD.WBP_RacingHUD_C"))
      (set `self.RacingHUD` _returnvalue)))
  (`UserWidget.AddToViewport` (`self.RacingHUD`) 0))

(fn `DrawRaceCompleteMenu`
  (`/Engine/EditorBlueprintResources/StandardMacros.IsValid` (`self.RaceCompleteMenu`)
    (:`Is Valid`
      _)
    (:`Is Not Valid`
      (bind _returnvalue (`|CreateWidget` "/Game/Class_Discuss/Blueprints/UI/WBP_RaceCompleteMenu.WBP_RaceCompleteMenu_C"))
      (set `self.RaceCompleteMenu` _returnvalue)))
  (`UserWidget.AddToViewport` (`self.RaceCompleteMenu`) 0))

(fn `GetStartingLine`
  (returns (StartingLine :type "/Game/Class_Discuss/Blueprints/BP_Startingline Object Reference") (bSuccess :type Boolean))
  (locals (StartingLineArray :type "Array of /Game/Class_Discuss/Blueprints/BP_Startingline Object Reference"))
  (bind _output (`|GetArrayItem` (`local.StartingLineArray`)))
  (`|ExecutionSequence`
    (:`then_0`
      (bind _outactors (`GameplayStatics.GetAllActorsOfClass` "/Game/Class_Discuss/Blueprints/BP_Startingline.BP_Startingline_C"))
      (set `local.StartingLineArray` _outactors))
    (:`then_1`
      ; Check if there is more than 1 starting line
      (if (> (`KismetArrayLibrary.Array_Length` (`local.StartingLineArray`)) 1)
        (`KismetSystemLibrary.PrintString` "Warning! There is more than one starting line in the level! Game mode may not work as expected!" true true (struct :`R` 1.0 :`G` 0.988697 :`B` 0.030844 :`A` 1.0))))
    (:`then_2`
      ; Check validity and return starting line
      (`/Engine/EditorBlueprintResources/StandardMacros.IsValid` _output
        (:`Is Valid`
          (return _output true))
        (:`Is Not Valid`
          (`KismetSystemLibrary.PrintString` "Error! No Starting line is present in level! Game will not function as intended!" true true (struct :`R` 1.0 :`G` 0.075002 :`A` 1.0) 99999999999.0)
          (return null false))))))

(fn `RecordLapTime`
  (bind _bp_timer (`self.BP_Timer`))
  (`KismetArrayLibrary.Array_Add` (`self.LapTimes`) (`/Game/Class_Discuss/Blueprints/BP_Timer.TotalTime (s)` _bp_timer))
  (`/Game/Class_Discuss/Blueprints/BP_Timer.ResetTimer` _bp_timer))

(fn `RemoveHUD`
  (`/Engine/EditorBlueprintResources/StandardMacros.IsValid` (`self.RacingHUD`)
    (:`Is Valid`
      (`Widget.RemoveFromParent` (`self.RacingHUD`)))))

(fn `UserConstructionScript`)