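; BP_Checkpoint is a racing checkpoint that records when a kart passes through it in sequence.
; Overlapping its CheckpointVolume with a BP_Kart sets CheckpointPassed only if PreviousCheckpoint has been passed, or if no valid previous checkpoint exists.
; It binds to the lap-completed event on BP_RacingGameMode to clear that flag each lap.
; The passed flag lives on the checkpoint itself rather than per kart.
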(event `self.ReceiveBeginPlay`
  (bind _asbp_racing_game_mode (cast `/Game/Class_Discuss/Blueprints/BP_RacingGameMode` (`GameplayStatics.GetGameMode`)))
  (add `/Game/Class_Discuss/Blueprints/BP_RacingGameMode.OnLapCompleted` _asbp_racing_game_mode (delegate `LapCompleted`)))

(event `LapCompleted`
  (set `self.bCheckpointPassed` false)
  (`KismetSystemLibrary.PrintString` "Checkpoint Reset!" true true (struct :`R` 1.0 :`G` 0.281498 :`A` 1.0)))

(event `self.CheckpointVolume.OnComponentBeginOverlap`
  (params (OverlappedComponent :type "PrimitiveComponent Object Reference") (OtherActor :type "Actor Object Reference") (OtherComp :type "PrimitiveComponent Object Reference") (OtherBodyIndex :type Integer) (bFromSweep :type Boolean) (SweepResult :type "HitResult Structure (by ref)"))
  (bind _previouscheckpoint (`self.PreviousCheckpoint`))
  (cast `/Game/Template/Blueprints/BP_Kart` OtherActor)
  (`/Engine/EditorBlueprintResources/StandardMacros.IsValid` _previouscheckpoint
    (:`Is Valid`
      (if (`/Game/Class_Discuss/Blueprints/BP_Checkpoint.bCheckpointPassed` _previouscheckpoint)
        (set `self.bCheckpointPassed` true :!label _label)))
    (:`Is Not Valid`
      (goto _label))))

(fn `UserConstructionScript`)