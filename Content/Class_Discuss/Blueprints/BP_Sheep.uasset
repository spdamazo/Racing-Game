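; BP_Sheep is a physics-driven actor with a goat mesh and a text render that shows random messages.
; On begin play and on every hit to the mesh, it picks a random entry from its message array for the text and jumps.
; Jump applies an impulse to the mesh along the normalized jump direction, scaled by jump force, so collisions keep it bouncing.
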(event `self.ReceiveBeginPlay`
  (bind (_message _output) (`self.GetRandomMessage`))
  (`TextRenderComponent.K2_SetText` (`self.TextRender`) _output)
  (`self.Jump`))

(event `self.SM_Goat.OnComponentHit`
  (params (HitComponent :type "PrimitiveComponent Object Reference") (OtherActor :type "Actor Object Reference") (OtherComp :type "PrimitiveComponent Object Reference") (NormalImpulse :type "Vector Structure") (Hit :type "HitResult Structure (by ref)"))
  (`self.Jump`)
  (bind (_message _output) (`self.GetRandomMessage`))
  (`TextRenderComponent.K2_SetText` (`self.TextRender`) _output))

(fn `GetRandomMessage`
  (returns (Message :type Text) (Output :type Text))
  (bind _message (`self.Message`))
  (return "" (`|GetArrayItem` _message (`KismetMathLibrary.RandomIntegerInRange` 0 (- (`KismetArrayLibrary.Array_Length` _message) 1)))))

(fn `Jump`
  (`PrimitiveComponent.AddImpulse` (`self.SM_Goat`) (* (`KismetMathLibrary.Normal` (`self.JumpDirection`)) (`self.JumpForce`)) "None" false))

(fn `UserConstructionScript`)