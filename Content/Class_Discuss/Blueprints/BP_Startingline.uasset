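; Starting line for a kart race that detects when a kart crosses it and reports whether the lap is complete.
; When a BP_Kart overlaps the checkpoint volume, it gathers all BP_Checkpoint actors except itself and checks that each is flagged as passed.
; It broadcasts the result through the OnStartingLinePassed dispatcher.
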(event `self.CheckpointVolume.OnComponentBeginOverlap`
  (params (OverlappedComponent :type "PrimitiveComponent Object Reference") (OtherActor :type "Actor Object Reference") (OtherComp :type "PrimitiveComponent Object Reference") (OtherBodyIndex :type Integer) (bFromSweep :type Boolean) (SweepResult :type "HitResult Structure (by ref)"))
  (cast `/Game/Template/Blueprints/BP_Kart` OtherActor)
  (bind _lapcompleted_ (`self.CheckLapCompletion`))
  (`self.OnStartingLinePassed` _lapcompleted_))

(fn `CheckLapCompletion`
  (returns (`LapCompleted?` :type Boolean))
  (locals (Checkpoints :type "Array of /Game/Class_Discuss/Blueprints/BP_Checkpoint Object Reference") (bLapCompleted :type Boolean))
  (`|ExecutionSequence`
    (:`then_0`
      (bind _outactors (`GameplayStatics.GetAllActorsOfClass` "/Game/Class_Discuss/Blueprints/BP_Checkpoint.BP_Checkpoint_C"))
      (bind _output_get (set `local.Checkpoints` _outactors))
      (`KismetArrayLibrary.Array_RemoveItem` _output_get self))
    (:`then_1`
      (set `local.bLapCompleted` true)
      (for _array_element (`local.Checkpoints`)
        (if (not (`/Game/Class_Discuss/Blueprints/BP_Checkpoint.bCheckpointPassed` _array_element))
          (set `local.bLapCompleted` false)
          (break))))
    (:`then_2`
      (return (`local.bLapCompleted`)))))

(fn `UserConstructionScript`
  (`parent.UserConstructionScript`))